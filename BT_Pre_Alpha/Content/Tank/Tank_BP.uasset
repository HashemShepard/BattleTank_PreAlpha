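; Player-controllable tank Blueprint that maps input to camera rotation, track-based driving and firing.
; Aim axes yaw a scene component and pitch the spring arm, FIRE calls Fire, and move axes feed MovementComp's OnWard and IntendTurnRight.
; Tick passes the barrel and turret to TankAim and both tracks to MovementComp, repeating this initialization every frame rather than at BeginPlay.
; Direct track Throttling calls are left unconnected.
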(event `self.ReceiveTick`
  (params (DeltaSeconds :type "Float (single-precision)"))
  (`TankAimComponent.intializeAim` (`self.TankAim`) (`self.TankBarrel`) (`self.Tank_Turret`))
  (`MovementComp.intialize` (`self.MovementComp`) (`self.LTankTracks`) (`self.RTankTracks`)))

(event `InputAxis|Aim Horizontal`
  (params (AxisValue :type "Float (single-precision)"))
  (`SceneComponent.K2_AddLocalRotation` (`self.Scene`) (`KismetMathLibrary.MakeRotator` 0.0 0.0 AxisValue) false false))

(event `InputAxis|Aim Vertical`
  (params (AxisValue :type "Float (single-precision)"))
  (`SceneComponent.K2_AddLocalRotation` (`self.SpringArm`) (`KismetMathLibrary.MakeRotator` 0.0 AxisValue) false false))

(event `InputAction|FIRE`
  (params (Key :type "Key Structure"))
  (:`Pressed`
    (`self.Fire`)))

(event `InputAxis|Move_Forward`
  (params (AxisValue :type "Float (single-precision)"))
  (`MovementComp.OnWard` (`self.MovementComp`) AxisValue))

(event `InputAxis|Move_Backward`
  (params (AxisValue :type "Float (single-precision)"))
  (`MovementComp.OnWard` (`self.MovementComp`) AxisValue))

(event `InputAxis|Move_Right`
  (params (AxisValue :type "Float (single-precision)"))
  (`MovementComp.IntendTurnRight` (`self.MovementComp`) AxisValue))

(event `InputAxis|Move_Left`
  (params (AxisValue :type "Float (single-precision)"))
  (`MovementComp.IntendTurnRight` (`self.MovementComp`) AxisValue))

(fn `UserConstructionScript`)